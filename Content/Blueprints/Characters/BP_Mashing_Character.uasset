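; Character for a button-mashing duel that plays a punch flipbook and shows the duel's outcome, driven by the GM_Mash_Duel game mode's phase.
; In one phase, Tick cycles static-mesh frames after a delay, decrementing SwingsRemaining.
; When swings run out, the winner shows victory and advances the phase while others show guard broken.
; In that next phase, non-winners switch to the defeated mesh.
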(event EventBeginPlay)

(event Collision|EventActorBeginOverlap
  (params (OtherActor :type Actor%20Object%20Reference)))

(event EventTick
  (params (DeltaSeconds :type Float%20%28single-precision%29))
  (bind _asgm_mash_duel (Utilities|Casting|CastToGM_Mash_Duel (Game|GetGameMode)))
  (if (Utilities|Enum|Equal(Enum) (Variables|/Game/Blueprints/GM_Mash_Duel.GM_Mash_Duel_C|GetGame%20Phase _asgm_mash_duel) "NewEnumerator3")
    (if (> (Variables|Default|GetSwings%20Remaining) 0)
      (Utilities|FlowControl|Delay (Variables|Default|GetPunching%20Delay))
      (Components|StaticMesh|SetStaticMesh (Variables|Default|GetCharacter%20Mesh) (Utilities|Array|Get(acopy) (Variables|Default|GetPunching%20Frames) (Variables|Default|GetPunch%20index)))
      (CallFunction|NextPunch)
      (else
        (Utilities|FlowControl|DoOnce false
          (:Completed
            (bind _asgm_mash_duel_2 (Utilities|Casting|CastToGM_Mash_Duel (Game|GetGameMode)))
            (if (== (Variables|/Game/Blueprints/GM_Mash_Duel.GM_Mash_Duel_C|GetWinner _asgm_mash_duel_2) self)
              (Components|StaticMesh|SetStaticMesh (Variables|Default|GetCharacter%20Mesh) "/Game/Assets/PlayerPoses/Player_Victory.Player_Victory")
              (bind _asgm_mash_duel_3 (Utilities|Casting|CastToGM_Mash_Duel (Game|GetGameMode)))
              (Variables|/Game/Blueprints/GM_Mash_Duel.GM_Mash_Duel_C|SetGame%20Phase _asgm_mash_duel_3 "NewEnumerator4")
              (else
                (Components|StaticMesh|SetStaticMesh (Variables|Default|GetCharacter%20Mesh) "/Game/Assets/PlayerPoses/Player_Guard_Broke.Player_Guard_Broke")))))))
    (elif (Utilities|Enum|Equal(Enum) (Variables|/Game/Blueprints/GM_Mash_Duel.GM_Mash_Duel_C|GetGame%20Phase _asgm_mash_duel) "NewEnumerator4")
      (Utilities|FlowControl|DoOnce false
        (:Completed
          (bind _asgm_mash_duel_4 (Utilities|Casting|CastToGM_Mash_Duel (Game|GetGameMode)))
          (if (not (== (Variables|/Game/Blueprints/GM_Mash_Duel.GM_Mash_Duel_C|GetWinner _asgm_mash_duel_4) self))
            (Components|StaticMesh|SetStaticMesh (Variables|Default|GetCharacter%20Mesh) "/Game/Assets/PlayerPoses/Player_Defeated.Player_Defeated")))))))

(fn ConstructionScript)

(fn IncreaseSwingCount
  (params (Swings :type Integer))
  (bind _output_get (Variables|Default|SetTotal%20Swing%20Count (+ Swings (Variables|Default|GetTotal%20Swing%20Count))))
  (Development|PrintString (Utilities|String|ToString(Integer) _output_get)))

(fn NextPunch
  (if (== (Variables|Default|GetPunch%20index) (- (Utilities|Array|Length (Variables|Default|GetPunching%20Frames)) 1))
    (Variables|Default|SetPunch%20index 0)
    (else
      (Variables|Default|SetPunch%20index (+ (Variables|Default|GetPunch%20index) 1))))
  (Math|Integer|DecrementInt (Variables|Default|GetSwings%20Remaining)))