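; BP_Player is the player-controlled character for a button-mash duel run by GM_Mash_Duel.
; It adds the IMC_Player Enhanced Input context on BeginPlay, and the first Ready press sets Readied and starts the game mode's countdown.
; Left and Right mash inputs feed TakeMashInput, which increases the swing count only when readied, in a specific game phase, and the input differs from the last counted one, enforcing alternation.
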(event Input|EnhancedActionEvents|EnhancedInputActionIA_Left_Mash
  (params (ActionValue :type Boolean) (ElapsedSeconds :type Float%20%28double-precision%29) (TriggeredSeconds :type Float%20%28double-precision%29) (InputAction :type Input%20Action%20Object%20Reference :default "/Game/Input/Actions/IA_Left_Mash.IA_Left_Mash"))
  (:Started
    (CallFunction|TakeMashInput "NewEnumerator1")))

(event Input|EnhancedActionEvents|EnhancedInputActionIA_Right_Mash
  (params (ActionValue :type Boolean) (ElapsedSeconds :type Float%20%28double-precision%29) (TriggeredSeconds :type Float%20%28double-precision%29) (InputAction :type Input%20Action%20Object%20Reference :default "/Game/Input/Actions/IA_Right_Mash.IA_Right_Mash"))
  (:Started
    (CallFunction|TakeMashInput "NewEnumerator2")))

(event Input|EnhancedActionEvents|EnhancedInputActionIA_Ready
  (params (ActionValue :type Boolean) (ElapsedSeconds :type Float%20%28double-precision%29) (TriggeredSeconds :type Float%20%28double-precision%29) (InputAction :type Input%20Action%20Object%20Reference :default "/Game/Input/Actions/IA_Ready.IA_Ready"))
  (:Started
    (if (not (Variables|Default|GetReadied))
      (Variables|Default|SetReadied true)
      (bind _asgm_mash_duel (Utilities|Casting|CastToGM_Mash_Duel (Game|GetGameMode)))
      (Default|StartCountdownEvent _asgm_mash_duel))))

(event EventBeginPlay
  (|CallParentFunction)
  (bind _asplayer_controller (Utilities|Casting|CastToPlayerController (Pawn|GetController)))
  (Input|AddMappingContext (PlayerController|LocalPlayerSubsystems|GetEnhancedInputLocalPlayerSubsystem _asplayer_controller) "/Game/Input/IMC_Player.IMC_Player" 0 "(bIgnoreAllPressedKeysUntilRelease=True,bForceImmediately=False)"))

(event Collision|EventActorBeginOverlap
  (params (OtherActor :type Actor%20Object%20Reference)))

(event EventTick
  (params (DeltaSeconds :type Float%20%28single-precision%29)))

(fn ConstructionScript
  (|CallParentFunction))

(fn TakeMashInput
  (params (Mash%20Input :type E_Input%20Enum :default "NewEnumerator0"))
  (if (Utilities|Enum|NotEqual(Enum) (Variables|Default|GetLast%20Input) Mash%20Input)
    (if (== true (Variables|Default|GetReadied))
      (bind _asgm_mash_duel (Utilities|Casting|CastToGM_Mash_Duel (Game|GetGameMode)))
      (if (Utilities|Enum|Equal(Enum) (Variables|/Game/Blueprints/GM_Mash_Duel.GM_Mash_Duel_C|GetGame%20Phase _asgm_mash_duel) "NewEnumerator2")
        (CallFunction|IncreaseSwingCount 1)
        (Variables|Default|SetLast%20Input Mash%20Input)))))