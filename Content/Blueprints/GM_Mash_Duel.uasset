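; GM_Mash_Duel is the game mode for a button-mashing duel between BP_Player and BP_Enemy.
; BeginPlay finds both actors and shows a ready-up widget, then StartCountdownEvent swaps it for a countdown widget.
; StartMashingEvent runs a timed mashing phase, advancing GamePhase, then PickWinner compares both SwingCounts and prints the result.
; A comment notes that the intended attack phase still lacks animations.
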(event Custom|Start%20Countdown%20Event
  (Variables|Default|SetGame%20Phase "NewEnumerator1")
  (bind _returnvalue (UserInterface|CreateWidget "/Game/Blueprints/WB_Countdown.WB_Countdown_C"))
  (Variables|Default|SetUI_Countdown _returnvalue)
  (UserInterface|Viewport|AddtoViewport _returnvalue 0)
  (Widget|SetVisibility (Variables|Default|GetUI_Ready) "Hidden"))

(event Custom|Start%20Mashing%20Event
  (Variables|Default|SetGame%20Phase "NewEnumerator2")
  (Utilities|FlowControl|Delay (Math|Conversions|ToFloat(Integer) (Variables|Default|GetMashing%20Time)))
  ;[1 1 1] Supposed to go to attacking we just dont have the animations and stuff for it
  (Variables|Default|SetGame%20Phase "NewEnumerator3")
  (CallFunction|PickWinner))

(event EventBeginPlay
  (bind _returnvalue (Actor|GetActorOfClass "/Game/Blueprints/Characters/BP_Player.BP_Player_C"))
  (Variables|Default|SetPlayer _returnvalue)
  (bind _returnvalue_2 (Actor|GetActorOfClass "/Game/Blueprints/Characters/BP_Enemy.BP_Enemy_C"))
  (Variables|Default|SetEnemy _returnvalue_2)
  (bind _returnvalue_3 (UserInterface|CreateWidget "/Game/Blueprints/WB_ReadyUp.WB_ReadyUp_C"))
  (Variables|Default|SetUI_Ready _returnvalue_3)
  (UserInterface|Viewport|AddtoViewport _returnvalue_3 0))

(event EventTick
  (params (DeltaSeconds :type Float%20%28single-precision%29)))

(fn ConstructionScript)

(fn PickWinner
  (Math|Float|CompareFloat (Math|Conversions|ToFloat(Integer) (Variables|/Game/Blueprints/Characters/BP_Mashing_Character.BP_Mashing_Character_C|GetSwing%20Count (Variables|Default|GetPlayer))) (Math|Conversions|ToFloat(Integer) (Variables|/Game/Blueprints/Characters/BP_Mashing_Character.BP_Mashing_Character_C|GetSwing%20Count (Variables|Default|GetEnemy)))
    (:>
      (Development|PrintString "Player Wins!"))
    (:==
      (Development|PrintString "Draw!"))
    (:<
      (Development|PrintString "Enemy Wins!"))))